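; BP_BaseCollectible is a base pickup actor that spins in place and is collected when the player or an NPC overlaps it.
; A looping timer rotates the root by a small yaw step, while sphere overlaps pass through CanBePickedUp, which accepts BP_FirstPersonCharacter or BP_NPC.
; OnPickUp plays a sound at the collector's location and destroys the actor.
; The construction script creates a dynamic material instance tinted by the Color variable.
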(event OnComponentBeginOverlap(SphereCollision)
  (params (OverlappedComponent :type Primitive%20Component%20Object%20Reference) (OtherActor :type Actor%20Object%20Reference) (OtherComp :type Primitive%20Component%20Object%20Reference) (OtherBodyIndex :type Integer) (bFromSweep :type Boolean) (SweepResult :type Hit%20Result%20Structure%20%28by%20ref%29))
  (bind _canbepicked (CallFunction|CanbePickedUp OtherActor))
  (if _canbepicked
    (CallFunction|OnPickUp OtherActor)))

(event Custom|On%20Pick%20Up
  (params (Character :type Actor%20Object%20Reference))
  ;[0.15 0.15 0.15 0.5] Xử lý khi đụng vào collectible
  (Audio|PlaySoundatLocation (Variables|Default|GetPickup%20Sound) (Transformation|GetActorLocation Character) "0, 0, 0" 1.0 1.0 0.0 0 0 0 0)
  (CallFunction|DestroyCollectible))

(event Custom|Destroy%20Collectible
  ;[0.15 0.15 0.15 0.5] Phá collectible. To-do: thêm hiệu ứng đẹp hơn
  (Actor|DestroyActor))

(event Custom|Rotate
  (Transformation|AddLocalRotation (Variables|Default|GetDefaultSceneRoot) (Math|Rotator|MakeRotator 0.0 0.0 0.5) false false))

(event EventBeginPlay
  (Utilities|Time|SetTimerbyEvent (delegate Custom|Rotate) 0.005 true))

(fn ConstructionScript
  (bind _returnvalue (Rendering|Material|CreateDynamicMaterialInstance (Variables|Default|GetStaticMesh) 0 "/Game/Collectible/Meshes/M_BaseCollectible_Inst.M_BaseCollectible_Inst" "None" :!class /Script/Engine.PrimitiveComponent))
  (bind _output_get (Variables|Default|SetMaterial _returnvalue))
  (Rendering|Material|SetVectorParameterValue _output_get "Color" (Variables|Default|GetColor) :!class /Script/Engine.MaterialInstanceDynamic))

(fn CanbePickedUp
  (params (Character :type Actor%20Object%20Reference))
  (Utilities|Casting|CastToBP_FirstPersonCharacter Character
    (:then
      (return true))
    (:CastFailed
      (Utilities|Casting|CastToBP_NPC Character
        (:then
          (return true))
        (:CastFailed
          (return false))))))