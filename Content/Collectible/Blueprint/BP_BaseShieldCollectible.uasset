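; Base shield pickup collectible that grants ShieldToAdd to the character that collects it.
; On pickup, a BP_FirstPersonCharacter gains shield through UpdateShieldByValue, while any other character gets the amount added to hit points, capped at maximum, via HitPoint message calls.
; CanBePickedUp extends the parent check by refusing first-person characters whose shield is already full; other characters need only pass the parent check.
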(event EventOnPickUp
  (params (Character :type Actor%20Object%20Reference))
  (|CallParentFunction Character)
  (bind _asbp_first_person_character (Utilities|Casting|CastToBP_FirstPersonCharacter Character)
    (:then
      (Default|UpdateShieldbyValue _asbp_first_person_character (Variables|Default|GetShieldToAdd)))
    (:CastFailed
      (bind (_current_hit_point _max_hit_point) (Class|BPIEnemyAI|GetHitPoint(Message) Character))
      (if (< (+ _current_hit_point (Variables|Default|GetShieldToAdd)) _max_hit_point)
        (Class|BPIEnemyAI|SetHitPoint(Message) Character (+ _current_hit_point (Variables|Default|GetShieldToAdd)) _max_hit_point)
        (else
          (Class|BPIEnemyAI|SetHitPoint(Message) Character _max_hit_point _max_hit_point))))))

(fn ConstructionScript
  (|CallParentFunction))

(fn CanbePickedUp
  (params (Character :type Actor%20Object%20Reference))
  (bind _canbepicked (|CallParentFunction Character))
  (if _canbepicked
    (bind _asbp_first_person_character (Utilities|Casting|CastToBP_FirstPersonCharacter Character)
      (:then
        (return (< (Variables|/Game/FirstPerson/Blueprints/BP_FirstPersonCharacter.BP_FirstPersonCharacter_C|GetShield _asbp_first_person_character) (Variables|/Game/FirstPerson/Blueprints/BP_FirstPersonCharacter.BP_FirstPersonCharacter_C|GetMaxShield _asbp_first_person_character))))
      (:CastFailed
        (return true)))
    (else
      (return false))))